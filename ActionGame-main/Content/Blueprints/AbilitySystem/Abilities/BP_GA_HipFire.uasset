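; Gameplay ability for hip-firing the equipped weapon automatically, activated only when there is enough ammo.
; It plays the weapon's attack montage and runs a looping timer at its fire rate, re-committing the ability on every shot.
; Each shot traces from weapon to focus, plays effects, decrements ammo and applies the weapon's gameplay effect to valid hit targets.
; An attack-ended gameplay event, montage end or failed commit ends the ability, clearing the timer.
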(event `self.K2_ActivateAbilityFromEvent`
  (params (EventData :type "GameplayEventData Structure (by ref)"))
  (bind _returnvalue (`self.GetEquippedItemWeaponStaticData`))
  (bind _returnvalue_2 (`self.K2_CommitAbility`))
  (if _returnvalue_2
    (`AbilityTask_PlayMontageAndWait.CreatePlayMontageAndWaitProxy` "None" (`WeaponStaticData.AttackMontage` _returnvalue)
      (:`then`
        (bind _returnvalue_3 (`KismetSystemLibrary.K2_SetTimerDelegate` (delegate `Shoot`) (/ 1.0 (`WeaponStaticData.FireRate` _returnvalue)) true))
        (set `self.ShootTimerHandle` _returnvalue_3)
        (`self.Shoot`)
        (`AbilityTask_WaitGameplayEvent.WaitGameplayEvent` (struct :`TagName` "Event.Combat.Attack.Ended") null true
          (:`EventReceived`
            (`self.K2_EndAbility`))))
      (:`OnCompleted`
        (`self.K2_EndAbility` :!label _label))
      (:`OnInterrupted`
        (goto _label))
      (:`OnCancelled`
        (goto _label)))
    (else
      (`self.K2_EndAbility`))))

(event `Shoot`
  (bind (_outhitresult _returnvalue) (`self.GetWeaponToFocusTraceResult` (`self.ShootingDistance`) "TraceTypeQuery3"))
  (bind _returnvalue_2 (`AbilitySystemBlueprintLibrary.GetAbilitySystemComponent` (`.HitActor` (`GameplayStatics.BreakHitResult` _outhitresult))))
  (bind _returnvalue_3 (`self.K2_CommitAbility`))
  (if _returnvalue_3
    (`WeaponItemActor.PlayWeaponEffects` (`self.GetEquippedWeaponItemActor`) _outhitresult)
    (`self.DecAmmo`)
    (if _returnvalue
      (`/Engine/EditorBlueprintResources/StandardMacros.IsValid` _returnvalue_2
        (:`Is Valid`
          (`AbilitySystemComponent.BP_ApplyGameplayEffectSpecToSelf` _returnvalue_2 (`self.GetWeaponEffectSpec` _outhitresult)))))
    (else
      (`self.K2_EndAbility`))))

(event `self.K2_OnEndAbility`
  (params (bWasCancelled :type Boolean))
  (`KismetSystemLibrary.K2_ClearAndInvalidateTimerHandle` (`self.ShootTimerHandle`)))

(fn `K2_CanActivateAbility`
  (params (ActorInfo :type "GameplayAbilityActorInfo Structure") (Handle :type "GameplayAbilitySpecHandle Structure"))
  (returns (RelevantTags :type "GameplayTagContainer Structure") (ReturnValue :type Boolean))
  (return (struct) (`self.HasEnoughAmmo`)))