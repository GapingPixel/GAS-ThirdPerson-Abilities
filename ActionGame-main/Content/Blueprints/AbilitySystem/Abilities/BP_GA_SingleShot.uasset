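; Gameplay ability for a single weapon shot, activatable only when there is enough ammo.
; After committing, it plays the equipped weapon's attack montage and fires on the Event.Combat.Shoot gameplay event, ending if the montage finishes or breaks off.
; The shot traces from weapon to focus, plays weapon effects, spends ammo and applies the weapon's effect spec to any hit actor's ability system, then ends the ability.
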(event `self.K2_ActivateAbilityFromEvent`
  (params (EventData :type "GameplayEventData Structure (by ref)"))
  (bind _returnvalue (`self.K2_CommitAbility`))
  (if _returnvalue
    (`AbilityTask_PlayMontageAndWait.CreatePlayMontageAndWaitProxy` "None" (`WeaponStaticData.AttackMontage` (`self.GetEquippedItemWeaponStaticData`))
      (:`then`
        (`AbilityTask_WaitGameplayEvent.WaitGameplayEvent` (struct :`TagName` "Event.Combat.Shoot") null true
          (:`EventReceived`
            (`self.Shoot`))))
      (:`OnCompleted`
        (`self.K2_EndAbility` :!label _label))
      (:`OnBlendOut`
        (goto _label))
      (:`OnInterrupted`
        (goto _label))
      (:`OnCancelled`
        (goto _label)))
    (else
      (`self.K2_EndAbility`))))

(event `Shoot`
  (bind (_outhitresult _returnvalue) (`self.GetWeaponToFocusTraceResult` (`self.ShootingDistance`) "TraceTypeQuery3"))
  (bind _returnvalue_2 (`AbilitySystemBlueprintLibrary.GetAbilitySystemComponent` (`.HitActor` (`GameplayStatics.BreakHitResult` _outhitresult))))
  (`WeaponItemActor.PlayWeaponEffects` (`self.GetEquippedWeaponItemActor`) _outhitresult)
  (`self.DecAmmo`)
  (if _returnvalue
    (`/Engine/EditorBlueprintResources/StandardMacros.IsValid` _returnvalue_2
      (:`Is Valid`
        (`AbilitySystemComponent.BP_ApplyGameplayEffectSpecToSelf` _returnvalue_2 (`self.GetWeaponEffectSpec` _outhitresult)))
      (:`Is Not Valid`
        _)))
  (`self.K2_EndAbility`))

(fn `K2_CanActivateAbility`
  (params (ActorInfo :type "GameplayAbilityActorInfo Structure") (Handle :type "GameplayAbilitySpecHandle Structure"))
  (returns (RelevantTags :type "GameplayTagContainer Structure") (ReturnValue :type Boolean))
  (return (struct) (`self.HasEnoughAmmo`)))